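; Sprint action Blueprint that raises its owning Character's walk speed while the action runs.
; On start it casts the Owner to Character and adds SpeedIncrease to the movement component's MaxWalkSpeed.
; On end it subtracts the same amount, adjusting speed relatively rather than caching and restoring the original value.
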(event `self.OnActionStart`
  (params (Instigator :type "Actor Object Reference"))
  (bind _ascharacter (cast `Character` (`self.Owner`)))
  (bind _charactermovement (`Character.CharacterMovement` _ascharacter))
  (set `CharacterMovementComponent.MaxWalkSpeed` (+ (`CharacterMovementComponent.MaxWalkSpeed` _charactermovement) (`self.SpeedIncrease`)) _charactermovement))

(event `self.OnActionEnd`
  (params (Instigator :type "Actor Object Reference"))
  (bind _ascharacter (cast `Character` (`self.Owner`)))
  (bind _charactermovement (`Character.CharacterMovement` _ascharacter))
  (set `CharacterMovementComponent.MaxWalkSpeed` (- (`CharacterMovementComponent.MaxWalkSpeed` _charactermovement) (`self.SpeedIncrease`)) _charactermovement))