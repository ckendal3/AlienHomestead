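; Minigun weapon Blueprint that auto-fires while the primary action is held.
; Pressing starts a looping timer at the time between shots and fires immediately, so taps always shoot; releasing clears the timer.
; Each shot, if no action is running, starts PrimaryAttack on the action component, then stops SpawnProjectile.
; Unequipping calls StopAction.
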(event `self.PrimaryAction`
  (params (bStart :type Boolean))
  (if bStart
    (bind _returnvalue (`KismetSystemLibrary.K2_SetTimerDelegate` (delegate `Fire`) (`self.TimeBetweenShoots`) true))
    (set `self.Handle_FireTimer` _returnvalue)
    ;[1 1 1] Always Fire on tapping
    (`self.Fire`)
    (else
      (`KismetSystemLibrary.K2_ClearAndInvalidateTimerHandle` (`self.Handle_FireTimer`)))))

(event `Fire`
  (if (not (`ActionComponent.HasRunningAction` (`self.ActionComponent`)))
    (`ActionComponent.StartAction` (`self.ActionComponent`) "PrimaryAttack" self)
    (`ActionComponent.StopAction` (`self.ActionComponent`) "SpawnProjectile" self)))

(event `self.OnUnequipped`
  (`self.StopAction` 0))

(fn `UserConstructionScript`)