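; Primary attack action for the player that fires a projectile toward the IsoShooterCharacter's aim location.
; On action start it spawns a BP_BaseProjectile rotated randomly within a narrow cone around that aim direction, then flips the active barrel.
; A custom start-location function returns the left or right barrel socket on BP_Player, falling back to the attach parent's location for other actors.
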(event `self.OnActionStart`
  (params (Instigator :type "Actor Object Reference"))
  (bind _returnvalue (`KismetMathLibrary.DegreesToRadians` 7.5))
  (bind _owner (`self.Owner`))
  (`/Engine/EditorBlueprintResources/StandardMacros.IsValid` _owner
    (:`Is Valid`
      (for _ (range 1)
        (`|SpawnActorFromClass` "/Game/Blueprints/Weapon/Projectiles/BP_BaseProjectile.BP_BaseProjectile_C" (`KismetMathLibrary.MakeTransform` (`self.GetStartLocation`) (`KismetMathLibrary.Conv_VectorToRotator` (`KismetMathLibrary.RandomUnitVectorInEllipticalConeInRadians` (`KismetMathLibrary.Conv_RotatorToVector` (`KismetMathLibrary.FindLookAtRotation` (`self.GetStartLocation`) (`IsoShooterCharacter.GetAimLocation` (cast `IsoShooterCharacter` (`Actor.GetAttachParentActor` _owner) :!pure true)))) _returnvalue _returnvalue))) "AlwaysSpawn" "OverrideRootScale" (`self.Owner`) (cast `Pawn` (`Actor.GetOwner` (`self.Owner`)) :!pure true))
        (set `self.bLeftBarrel` (not (`self.bLeftBarrel`)))))))

(fn `GetStartLocation_Custom`
  (returns (ReturnValue :type "Vector Structure"))
  (bind _asbp_player (cast `/Game/Blueprints/Player/BP_Player` (`Actor.GetAttachParentActor` (`self.Owner`)))
    (:`then`
      (return (`SceneComponent.GetSocketLocation` (`Character.Mesh` _asbp_player) (select `bool` (`self.bLeftBarrel`) :`false` "barrel_r" :`true` "barrel_l" :!type "Name"))))
    (:`CastFailed`
      (return (`Actor.K2_GetActorLocation` (`Actor.GetAttachParentActor` (`self.Owner`)))))))