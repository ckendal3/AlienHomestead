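; BP_KillField is an area hazard that deals repeated damage to SpiderMinion characters inside it.
; OverlapComponent begin and end events add and remove minions from CharacterArray.
; A looping timer started on BeginPlay applies fixed damage to every tracked minion several times a second.
; The timer event is named HealPlayers, although it only damages minions.
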(event `self.ReceiveBeginPlay`
  (`KismetSystemLibrary.K2_SetTimerDelegate` (delegate `HealPlayers`) 0.25 true))

(event `HealPlayers`
  (for _array_element (`self.CharacterArray`)
    (`GameplayStatics.ApplyDamage` _array_element 25.0 null self)))

(event `self.OverlapComponent.OnComponentBeginOverlap`
  (params (OverlappedComponent :type "PrimitiveComponent Object Reference") (OtherActor :type "Actor Object Reference") (OtherComp :type "PrimitiveComponent Object Reference") (OtherBodyIndex :type Integer) (bFromSweep :type Boolean) (SweepResult :type "HitResult Structure (by ref)"))
  (bind _asspider_minion (cast `SpiderMinion` OtherActor))
  (`KismetArrayLibrary.Array_AddUnique` (`self.CharacterArray`) _asspider_minion))

(event `self.OverlapComponent.OnComponentEndOverlap`
  (params (OverlappedComponent :type "PrimitiveComponent Object Reference") (OtherActor :type "Actor Object Reference") (OtherComp :type "PrimitiveComponent Object Reference") (OtherBodyIndex :type Integer))
  (bind _asspider_minion (cast `SpiderMinion` OtherActor))
  (`KismetArrayLibrary.Array_RemoveItem` (`self.CharacterArray`) _asspider_minion))

(fn `UserConstructionScript`)