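; Behavior Tree task that picks the nearest attackable target for an AI-controlled pawn.
; On execute, it rebuilds an array of every IsoShooterCharacter and DefendableBase actor in the world.
; It writes the actor nearest the pawn to a Blackboard key, then finishes with success only if that actor is valid.
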(event `self.ReceiveExecuteAI`
  (params (OwnerController :type "AIController Object Reference") (ControlledPawn :type "Pawn Object Reference"))
  (bind (_distance _returnvalue) (`GameplayStatics.FindNearestActor` (`Actor.K2_GetActorLocation` ControlledPawn) (`self.ActorArray`)))
  (`KismetArrayLibrary.Array_Clear` (`self.ActorArray`))
  (`|ExecutionSequence`
    (:`then_0`
      (bind _outactors (`GameplayStatics.GetAllActorsOfClass` "/Script/AlienHomestead.IsoShooterCharacter"))
      (`KismetArrayLibrary.Array_Append` (`self.ActorArray`) _outactors))
    (:`then_1`
      (bind _outactors_2 (`GameplayStatics.GetAllActorsOfClass` "/Script/AlienHomestead.DefendableBase"))
      (`KismetArrayLibrary.Array_Append` (`self.ActorArray`) _outactors_2))
    (:`then_2`
      (`BTFunctionLibrary.SetBlackboardValueAsObject` (`self.Key`) _returnvalue)
      (`self.FinishExecute` (`KismetSystemLibrary.IsValid` _returnvalue)))))